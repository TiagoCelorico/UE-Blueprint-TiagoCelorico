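; BP_SlidingDoor is an interactable door that slides from its starting position to a marked end position.
; BeginPlay caches the world locations of the mesh and the EndPositionMarker component as the two endpoints.
; Interact plays a Timeline that lerps the mesh between them without sweeping, with no reverse path to close it.
; CanInteract always returns true, whoever the instigator is.
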(event `self.ReceiveBeginPlay`
  (set `self.InitialPosition` (`SceneComponent.K2_GetComponentLocation` (`self.StaticMeshComponent`)))
  (set `self.FinalPosition` (`SceneComponent.K2_GetComponentLocation` (`self.EndPosition marker`))))

(event `/Game/BPI_Interactable.Interact`
  (params (Instigator :type "Actor Object Reference"))
  (bind (_direction _lerptime) (`Timeline|Timeline`)
    (:`Update`
      (`SceneComponent.K2_SetWorldLocation` (`self.StaticMeshComponent`) (`KismetMathLibrary.VLerp` (`self.InitialPosition`) (`self.FinalPosition`) _lerptime) false false))))

(fn `CanInteract`
  (params (Instigator :type "Actor Object Reference"))
  (returns (State :type Boolean))
  (return true))

(fn `UserConstructionScript`)