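; BP_HealthComponent is a health component that tracks current and maximum health and broadcasts healed, damaged and died events.
; On BeginPlay it can optionally fill health to max, then waits a tick before broadcasting the heal.
; ModifyHealth applies a signed delta without clamping, calling OnDied at zero or below, otherwise OnHealed or OnDamaged with normalized health.
; Damage amounts are passed as negative values.
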(event `self.ReceiveBeginPlay`
  (if (`self.ShouldSetCUrrentHealthToMaxHealth`)
    (set `self.CurrentHealth` (`self.MaxHealth`))
    (`KismetSystemLibrary.DelayUntilNextTick`)
    (`self.OnHealed` (`self.MaxHealth`) (`self.GetNormalizedHealth`))))

(fn `GetNormalizedHealth`
  (returns (NormalizedHealth :type "Float (double-precision)"))
  (return (`KismetMathLibrary.SafeDivide` (`self.CurrentHealth`) (`self.MaxHealth`))))

(fn `ModifyHealth`
  (params (DeltaChange :type "Float (double-precision)"))
  (bind _normalizedhealth (`self.GetNormalizedHealth`))
  (bind _deltachange (`local.DeltaChange`))
  (bind _output_get (set `self.CurrentHealth` (+ DeltaChange (`self.CurrentHealth`))))
  (if (<= _output_get 0.0)
    (`self.OnDied`)
    (elif (> (`local.DeltaChange`) 0.0)
      (`self.OnHealed` _deltachange _normalizedhealth)
      (elif (< (`local.DeltaChange`) 0.0)
        (`self.OnDamaged` _deltachange _normalizedhealth)))))