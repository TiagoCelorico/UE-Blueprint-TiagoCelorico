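; BP_Interactor finds the interactable object the player camera looks at and forwards interaction requests to it.
; Each Tick, a Visibility sphere trace with persistent debug drawing runs along the camera forward vector, storing hit actors implementing BPI_Interactable in ObjectToInteract or clearing it.
; RequestInteract validates instigator and target, calls CanInteract, then calls Interact regardless of that result, returning whether it ran.
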(event `self.ReceiveTick`
  (params (DeltaSeconds :type "Float (single-precision)"))
  (bind _returnvalue (`GameplayStatics.GetPlayerCameraManager` 0))
  (bind _returnvalue_2 (`Actor.K2_GetActorLocation` _returnvalue))
  (bind (_outhit _returnvalue_3) (`KismetSystemLibrary.SphereTraceSingle` :`Start` _returnvalue_2 :`End` (+ _returnvalue_2 (* (`Actor.GetActorForwardVector` _returnvalue) (`self.RayDIstance`))) :`TraceChannel` "TraceTypeQuery1" :`DrawDebugType` "Persistent"))
  (if _returnvalue_3
    (bind (_bblockinghit _binitialoverlap _time _distance _location _impactpoint _normal _impactnormal _physmat _hitactor) (`GameplayStatics.BreakHitResult` _outhit))
    (if (`KismetSystemLibrary.DoesImplementInterface` _hitactor "/Game/BPI_Interactable.BPI_Interactable_C")
      (if (not (== (`self.ObjectToInteract`) _hitactor))
        (set `self.ObjectToInteract` _hitactor))
      (else
        (set `self.ObjectToInteract` null :!label _label)))
    (else
      (goto _label))))

(fn `RequestInteract`
  (params (Instigator :type "Actor Object Reference"))
  (returns (WasSuccessfull :type Boolean))
  (locals (NewLocalVar :type "/Game/BPI_Interactable Interface"))
  (`/Engine/EditorBlueprintResources/StandardMacros.IsValid` Instigator
    (:`Is Valid`
      (`/Engine/EditorBlueprintResources/StandardMacros.IsValid` (`self.ObjectToInteract`)
        (:`Is Valid`
          (message `/Game/BPI_Interactable.CanInteract` (`self.ObjectToInteract`) (`local.Instigator`))
          (if true
            (message `/Game/BPI_Interactable.Interact` (`self.ObjectToInteract`) (`local.Instigator`))
            (return true)
            (else
              _)))
        (:`Is Not Valid`
          _)))
    (:`Is Not Valid`
      _))
  (return false))